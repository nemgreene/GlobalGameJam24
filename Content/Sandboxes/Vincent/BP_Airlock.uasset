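; BP_Airlock is an airlock actor that tells the game mode when the player character enters it.
; Overlap on the BC component filters for TP_SpaceGirl02_CR, then passes the airlock to EnterAirlock on BP_GameMode_VG.
; ToggleFields is currently a no-op: its logic for switching visibility and collision on the Start and End fields is disconnected.
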(event `self.BC.OnComponentBeginOverlap`
  (params (OverlappedComponent :type "PrimitiveComponent Object Reference") (OtherActor :type "Actor Object Reference") (OtherComp :type "PrimitiveComponent Object Reference") (OtherBodyIndex :type Integer) (bFromSweep :type Boolean) (SweepResult :type "HitResult Structure (by ref)"))
  (cast `/Game/Sandboxes/Clayton/C_BluePrints/SpaceGirl/TP_SpaceGirl02_CR` OtherActor)
  (bind _asbp_game_mode_vg (cast `/Game/Sandboxes/Vincent/BP_GameMode_VG` (`GameplayStatics.GetGameMode`)))
  (`/Game/Sandboxes/Vincent/BP_GameMode_VG.Enter Airlock` _asbp_game_mode_vg self))

(fn `ToggleFields`
  (params (Active :type Boolean)))

(fn `UserConstructionScript`)